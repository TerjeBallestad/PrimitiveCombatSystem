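; Talent grid cell actor that displays a talent's base type on each of its four sides: North, South, East and West.
; Setup stores the grid coordinate and the slot and talent names from CellData, then sets each side's material from TalentData.
; BaseTypeToMaterial maps each base type to a material, with All sharing the Light material and None returning no material.
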(event EventBeginPlay)

(event Collision|EventActorBeginOverlap
  (params (OtherActor :type Actor%20Object%20Reference)))

(event EventTick
  (params (DeltaSeconds :type Float%20%28single-precision%29)))

(fn ConstructionScript)

(fn Setup
  (params (CellData :type Talent%20Grid%20Cell%20Structure) (TalentData :type Talent%20Data%20Structure) (Coordinate :type Int%20Point%20Structure))
  (Variables|Default|SetCoordinate Coordinate)
  (Variables|Default|SetCell%20Data%20Slot%20Name (.slotname CellData))
  (Variables|Default|SetCell%20Data%20Talent%20Name (.talentname CellData))
  (Utilities|FlowControl|Sequence
    (:then_0
      (Rendering|Material|SetMaterial (Variables|Default|GetSouth) 0 (CallFunction|BaseTypetoMaterial (.south TalentData))))
    (:then_1
      (Rendering|Material|SetMaterial (Variables|Default|GetNorth) 0 (CallFunction|BaseTypetoMaterial (.north TalentData))))
    (:then_2
      (Rendering|Material|SetMaterial (Variables|Default|GetEast) 0 (CallFunction|BaseTypetoMaterial (.east TalentData))))
    (:then_3
      (Rendering|Material|SetMaterial (Variables|Default|GetWest) 0 (CallFunction|BaseTypetoMaterial (.west TalentData))))))

(fn BaseTypetoMaterial
  (params (BaseType :type EBaseType%20Enum :default "N"))
  (switch Utilities|FlowControl|Switch|SwitchonEBaseType BaseType
    (:N
      (return 0))
    (:L
      (return (Variables|Default|GetLightMaterial)))
    (:B
      (return (Variables|Default|GetBlueMaterial)))
    (:D
      (return (Variables|Default|GetDarkMaterial)))
    (:R
      (return (Variables|Default|GetRedMaterial)))
    (:G
      (return (Variables|Default|GetGreenMaterial)))
    (:A
      (return (Variables|Default|GetLightMaterial)))))