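; Actor that builds a character's talent grid in the world at BeginPlay from its CharacterGrids data table row.
; It takes grid bounds from the last map key, then spawns BP_TalentGridCell actors around an offset origin, with both dimensions derived from Rows.
; Each cell is set up with its TalentData row, looked up by slot name.
; It also creates five colored dynamic instances of M_GridBase, which are not applied here.
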(event EventBeginPlay
  (bind _returnvalue (Utilities|GetDataTableRow (Variables|Default|GetCharacterGrids) (Variables|Default|GetCharacter%20Name))
    (:then
      (bind _structout (Utilities|Struct|SetmembersinTalentGridCharacter _returnvalue))
      (Variables|Default|SetStruct%20Out _structout)
      (CallFunction|CreateMaterialInstances "(R=1.000000,G=0.923859,B=0.406250,A=1.000000)" "(R=0.154568,G=0.339337,B=0.802083,A=1.000000)" "(R=0.276371,G=0.036448,B=0.453125,A=1.000000)" "(R=0.802083,G=0.115139,B=0.163052,A=1.000000)" "(R=0.251720,G=0.864583,B=0.144097,A=1.000000)")
      (bind _keys (Utilities|Map|Keys (.grid (Variables|Default|GetStruct%20Out))))
      (bind _output_get (Variables|Default|SetCollumns (.x (Utilities|Array|Get(acopy) _keys (- (Utilities|Map|Length (.grid (Variables|Default|GetStruct%20Out))) 1)))))
      (bind _output_get_2 (Variables|Default|SetRows (.y (Utilities|Array|Get(acopy) _keys (- (Utilities|Map|Length (.grid (Variables|Default|GetStruct%20Out))) 1)))))
      (bind _result (Math|Float|NegateFloat (CallFunction|GetWidth))
        (:%20%20
          (bind _result_2 (Math|Float|NegateFloat (CallFunction|GetHeight))
            (:%20%20
              (Variables|Default|SetOrigin (Math|Vector|MakeVector (/ _result 2.0) (/ _result_2 2.0) 0.0))
              (for _index (range 0 _output_get_2)
                (for _index_2 (range 0 _output_get)
                  (CallFunction|CreateCell (+ (Math|Vector|MakeVector (* _index (Variables|Default|GetCellWidth)) (* _index_2 (Variables|Default|GetCellHeight)) 0.0) (Variables|Default|GetOrigin)) (.Value (Utilities|Map|Find (.grid (Variables|Default|GetStruct%20Out)) (Utilities|Struct|MakeIntPoint _index _index_2)))))))))))))

(event Collision|EventActorBeginOverlap
  (params (OtherActor :type Actor%20Object%20Reference)))

(event EventTick
  (params (DeltaSeconds :type Float%20%28single-precision%29)))

(fn ConstructionScript)

(fn CreateMaterialInstances
  (params (LightColor :type Linear%20Color%20Structure) (BlueColor :type Linear%20Color%20Structure) (DarkColor :type Linear%20Color%20Structure) (RedColor :type Linear%20Color%20Structure) (GreenColor :type Linear%20Color%20Structure))
  (Utilities|FlowControl|Sequence
    (:then_0
      (bind _returnvalue (Rendering|Material|CreateDynamicMaterialInstance "/Game/TalentGrid/M_GridBase.M_GridBase" "None" "None" :!class /Script/Engine.KismetMaterialLibrary))
      (bind _output_get (Variables|Default|SetLightMaterial _returnvalue))
      (Rendering|Material|SetVectorParameterValue _output_get "Color" LightColor :!class /Script/Engine.MaterialInstanceDynamic))
    (:then_1
      (bind _returnvalue_2 (Rendering|Material|CreateDynamicMaterialInstance "/Game/TalentGrid/M_GridBase.M_GridBase" "None" "None" :!class /Script/Engine.KismetMaterialLibrary))
      (bind _output_get_2 (Variables|Default|SetBlueMaterial _returnvalue_2))
      (Rendering|Material|SetVectorParameterValue _output_get_2 "Color" BlueColor :!class /Script/Engine.MaterialInstanceDynamic))
    (:then_2
      (bind _returnvalue_3 (Rendering|Material|CreateDynamicMaterialInstance "/Game/TalentGrid/M_GridBase.M_GridBase" "None" "None" :!class /Script/Engine.KismetMaterialLibrary))
      (bind _output_get_3 (Variables|Default|SetDarkMaterial _returnvalue_3))
      (Rendering|Material|SetVectorParameterValue _output_get_3 "Color" DarkColor :!class /Script/Engine.MaterialInstanceDynamic))
    (:then_3
      (bind _returnvalue_4 (Rendering|Material|CreateDynamicMaterialInstance "/Game/TalentGrid/M_GridBase.M_GridBase" "None" "None" :!class /Script/Engine.KismetMaterialLibrary))
      (bind _output_get_4 (Variables|Default|SetRedMaterial _returnvalue_4))
      (Rendering|Material|SetVectorParameterValue _output_get_4 "Color" RedColor :!class /Script/Engine.MaterialInstanceDynamic))
    (:then_4
      (bind _returnvalue_5 (Rendering|Material|CreateDynamicMaterialInstance "/Game/TalentGrid/M_GridBase.M_GridBase" "None" "None" :!class /Script/Engine.KismetMaterialLibrary))
      (bind _output_get_5 (Variables|Default|SetGreenMaterial _returnvalue_5))
      (Rendering|Material|SetVectorParameterValue _output_get_5 "Color" GreenColor :!class /Script/Engine.MaterialInstanceDynamic))))

(fn CreateCell
  (params (Location :type Vector) (CellData :type Talent%20Grid%20Cell%20Structure))
  (bind _returnvalue (Game|SpawnActorfromClass "/Game/TalentGrid/BP_TalentGridCell.BP_TalentGridCell_C" (Math|Transform|MakeTransform Location "0, 0, 0" "1,1,1") "Undefined" 0 0))
  (Utilities|Array|Add (Variables|Default|GetCells) _returnvalue)
  (bind _returnvalue_2 (Utilities|GetDataTableRow (Variables|Default|GetTalentData) (Utilities|String|StringToName (.slotname CellData)))
    (:then
      (bind _structout (Utilities|Struct|SetmembersinTalentData _returnvalue_2))
      (Default|Setup _returnvalue (Utilities|Struct|MakeTalentGridCell (.slotname CellData) (.talentname CellData)) _structout))))

(fn GetHeight
  (return (* (Variables|Default|GetRows) (Variables|Default|GetCellHeight))))

(fn GetWidth
  (return (* (Variables|Default|GetRows) (Variables|Default|GetCellWidth))))