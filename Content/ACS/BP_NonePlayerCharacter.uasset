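; BP_NonePlayerCharacter is an NPC character with overhead widgets for cast bar, health bar and floating damage text.
; On BeginPlay it registers with BP_GameState and caches those widgets, filling the cast bar from the cast timer while casting.
; Entering combat has the game state disable other NPCs and passes the enemy to BP_NonePlayerController as target.
; It can cast a random spell from its character data.
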(event Custom|UpdateCastBar
  (bind _casttimehandle (Variables|Default|GetCastTimeHandle))
  (bind _returnvalue (Class|KismetSystemLibrary|GetTimerElapsedTimeHandle _casttimehandle))
  ;[1 1 1] Update Cast bar
  (Progress|SetPercent (Variables|/Game/ACS/UW_CastBar.UW_CastBar_C|GetCastBar (Variables|Default|GetCast%20Bar%20WIdget)) (/ _returnvalue (+ _returnvalue (Utilities|Time|GetTimerRemainingTimebyHandle _casttimehandle)))))

(event EventBeginPlay
  (bind _castbar (Variables|Default|GetCastBar))
  (bind _asbp_game_state (Utilities|Casting|CastToBP_GameState (Game|GetGameState)))
  (Utilities|Array|Add (Variables|/Game/ACS/BP_GameState.BP_GameState_C|GetNPCs _asbp_game_state) self)
  (bind _asuw_cast_bar (Utilities|Casting|CastToUW_CastBar (UserInterface|GetUserWidgetObject _castbar)))
  (Variables|Default|SetCast%20Bar%20WIdget _asuw_cast_bar)
  (Development|SetHiddeninGame _castbar true false)
  (bind _asuw_health_bar (Utilities|Casting|CastToUW_HealthBar (UserInterface|GetUserWidgetObject (Variables|Default|GetHealthBar))))
  (Variables|Default|SetHealth%20Bar%20Widget _asuw_health_bar)
  (bind _asuw_floating_combat_text (Utilities|Casting|CastToUW_FloatingCombatText (UserInterface|GetUserWidgetObject (Variables|Default|GetFloatingText))))
  (Variables|Default|SetFloating%20Text%20Widget _asuw_floating_combat_text))

(event EventEnteringCombat
  (params (Enemy :type ACS%20Character%20Object%20Reference))
  (|CallParentFunction Enemy)
  (Development|PrintString "Entering Combat")
  (bind _asbp_game_state (Utilities|Casting|CastToBP_GameState (Game|GetGameState)))
  (Default|DisableOtherNPCs _asbp_game_state self)
  (bind _asbp_none_player_controller (Utilities|Casting|CastToBP_NonePlayerController (Pawn|GetController)))
  (Default|SetTarget _asbp_none_player_controller Enemy))

(event EventTick
  (params (DeltaSeconds :type Float%20%28single-precision%29))
  (if (Variables|Default|GetIsCasting)
    (CallFunction|UpdateCastBar)))

(event EventUpdateHealthBar
  (Progress|SetPercent (Variables|/Game/ACS/UW_HealthBar.UW_HealthBar_C|GetProgressBar_0 (Variables|Default|GetHealth%20Bar%20Widget)) (/ (Class|ACSCharacter|GetCurrentHealth) (Class|ACSCharacter|GetMaxHealth))))

(event EventSpellCastEnd
  ;[1 0.2419 0.4023] Spell cast end
  (Development|SetHiddeninGame (Variables|Default|GetCastBar) true false))

(event EventSpellCastStart
  ;[0.9367 0.3612 1] Spell cast start
  (Development|SetHiddeninGame (Variables|Default|GetCastBar) false false))

(fn ConstructionScript)

(fn StartCastingRandomSpell
  (bind _characterdata (Variables|Default|GetCharacterData))
  (Class|ACSCharacter|CastSpell (Utilities|Array|Get(acopy) (.spells _characterdata) (Math|Random|RandomIntegerinRange 0 (- (Utilities|Array|Length (.spells _characterdata)) 1))))
  (return true))

(fn TakeDamage
  (params (DamageAmount :type Float%20%28single-precision%29) (DamageEvent :type Damage%20Event%20Structure%20%28by%20ref%29) (EventInstigator :type Controller%20Object%20Reference) (DamageCauser :type Actor%20Object%20Reference))
  (bind _floating_text_widget (Variables|Default|GetFloating%20Text%20Widget))
  (bind _returnvalue (|CallParentFunction DamageAmount DamageEvent EventInstigator DamageCauser))
  (Rendering|Components|TextRender|SetText (Variables|/Game/ACS/UW_FloatingCombatText.UW_FloatingCombatText_C|GetDamage _floating_text_widget) (Utilities|Text|ToText(Float) _returnvalue "HalfToEven"))
  (Default|PlayFloatingAnimation _floating_text_widget)
  (return _returnvalue))