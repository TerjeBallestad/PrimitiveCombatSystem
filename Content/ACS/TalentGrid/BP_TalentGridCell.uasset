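; Actor for one cell of the talent grid, showing a slot and the talent placed in it.
; Setup stores the coordinate and, for visible cells, hides the cover, toggles the trauma rock and sets the talent's billboard sprite.
; Four directional meshes take materials from the slot's colour types.
; Talent meshes appear for non-empty directions, using emissive materials where the talent's type matches the slot's.
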(event EventBeginPlay)

(event Collision|EventActorBeginOverlap
  (params (OtherActor :type Actor%20Object%20Reference)))

(event EventTick
  (params (DeltaSeconds :type Float%20%28single-precision%29)))

(fn ConstructionScript)

(fn Setup
  (params (CellData :type Talent%20Grid%20Cell%20Structure) (TalentData :type Talent%20Data%20Structure) (Coordinate :type Int%20Point%20Structure) (SlotData :type Talent%20Slot%20Data%20Structure))
  (bind _billboard (Variables|Default|GetBillboard))
  (Variables|Default|SetCoordinate Coordinate)
  (Variables|Default|SetCell%20Data%20Slot%20Name (.slotname CellData))
  (Variables|Default|SetCell%20Data%20Talent%20Name (.talentname CellData))
  (if (.visible CellData)
    (Rendering|SetVisibility (Variables|Default|GetHidden) false false)
    (CallFunction|SetCardinalSlotMaterials SlotData)
    (Rendering|SetVisibility (Variables|Default|GetTraumaRock) (.trauma CellData) false)
    (CallFunction|SetCardinaTalentlMaterials TalentData SlotData)
    (Rendering|Components|Sprite|SetSprite _billboard (.Image (Utilities|Struct|BreakTalentData TalentData)))
    (Rendering|SetVisibility _billboard true false)))

(fn BaseTypetoMaterial
  (params (BaseType :type EBaseType%20Enum :default "N") (Emissive :type Boolean))
  (switch Utilities|FlowControl|Switch|SwitchonEBaseType BaseType
    (:N
      (return 0))
    (:L
      (if Emissive
        (return (Variables|Default|GetLightMaterial_Emissive))
        (else
          (return (Variables|Default|GetLightMaterial)))))
    (:B
      (if Emissive
        (return (Variables|Default|GetBlueMaterial_Emissive))
        (else
          (return (Variables|Default|GetBlueMaterial)))))
    (:D
      (if Emissive
        (return (Variables|Default|GetDarkMaterial_Emissive))
        (else
          (return (Variables|Default|GetDarkMaterial)))))
    (:R
      (if Emissive
        (return (Variables|Default|GetRedMaterial_Emissive))
        (else
          (return (Variables|Default|GetRedMaterial)))))
    (:G
      (if Emissive
        (return (Variables|Default|GetGreenMaterial_Emissive))
        (else
          (return (Variables|Default|GetGreenMaterial)))))
    (:A
      (return (Variables|Default|GetLightMaterial)))))

(fn SetCardinalSlotMaterials
  (params (SlotData :type Talent%20Slot%20Data%20Structure))
  (Utilities|FlowControl|Sequence
    (:then_0
      (Rendering|Material|SetMaterial (Variables|Default|GetNorth) 0 (CallFunction|BaseTypetoMaterial (.north SlotData) false)))
    (:then_1
      (Rendering|Material|SetMaterial (Variables|Default|GetEast) 0 (CallFunction|BaseTypetoMaterial (.east SlotData) false)))
    (:then_2
      (Rendering|Material|SetMaterial (Variables|Default|GetSouth) 0 (CallFunction|BaseTypetoMaterial (.south SlotData) false)))
    (:then_3
      (Rendering|Material|SetMaterial (Variables|Default|GetWest) 0 (CallFunction|BaseTypetoMaterial (.west SlotData) false)))))

(fn SetCardinaTalentlMaterials
  (params (TalentData :type Talent%20Data%20Structure) (SlotData :type Talent%20Slot%20Data%20Structure))
  (bind _talentnorth (Variables|Default|GetTalentNorth))
  (bind _talenteast (Variables|Default|GetTalentEast))
  (bind _talentsouth (Variables|Default|GetTalentSouth))
  (bind _talentwest (Variables|Default|GetTalentWest))
  (Utilities|FlowControl|Sequence
    (:then_0
      (if (!= (.north TalentData) 0)
        (Rendering|SetVisibility _talentnorth true false)
        (Rendering|Material|SetMaterial _talentnorth 0 (CallFunction|BaseTypetoMaterial (.north TalentData) (== (.north SlotData) (.north TalentData))))))
    (:then_1
      (if (!= (.east TalentData) 0)
        (Rendering|Material|SetMaterial _talenteast 0 (CallFunction|BaseTypetoMaterial (.east TalentData) (== (.east TalentData) (.east SlotData))))
        (Rendering|SetVisibility _talenteast true false)))
    (:then_2
      (if (!= (.south TalentData) 0)
        (Rendering|SetVisibility _talentsouth true false)
        (Rendering|Material|SetMaterial _talentsouth 0 (CallFunction|BaseTypetoMaterial (.south TalentData) (== (.south TalentData) (.south SlotData))))))
    (:then_3
      (if (!= (.west TalentData) 0)
        (Rendering|SetVisibility _talentwest true false)
        (Rendering|Material|SetMaterial _talentwest 0 (CallFunction|BaseTypetoMaterial (.west TalentData) (== (.west TalentData) (.west SlotData))))))))