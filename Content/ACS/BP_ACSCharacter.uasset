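; Player character Blueprint for the ACS system that handles the spell-casting HUD.
; On BeginPlay it creates a cast bar widget and adds a reticle widget to the viewport.
; SpellCastStart and SpellCastEnd events show and remove the cast bar.
; While IsCasting is true, Tick fills the bar from the cast timer handle's elapsed time over elapsed plus remaining time.
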(event Custom|UpdateCastBar
  (bind _casttimehandle (Variables|Default|GetCastTimeHandle))
  ;[1 1 1] Update cast bar
  (Progress|SetPercent (Variables|/Game/ACS/UW_CastBar.UW_CastBar_C|GetCastBar (Variables|Default|GetCastBar)) (/ (Class|KismetSystemLibrary|GetTimerElapsedTimeHandle _casttimehandle) (+ (Class|KismetSystemLibrary|GetTimerElapsedTimeHandle _casttimehandle) (Utilities|Time|GetTimerRemainingTimebyHandle _casttimehandle)))))

(event EventBeginPlay
  (bind _returnvalue (Game|GetPlayerController 0))
  (bind _returnvalue_2 (UserInterface|CreateWidget "/Game/ACS/UW_CastBar.UW_CastBar_C" _returnvalue))
  (Variables|Default|SetCastBar _returnvalue_2)
  (bind _returnvalue_3 (UserInterface|CreateWidget "/Game/ACS/UW_Reticle.UW_Reticle_C" _returnvalue))
  (UserInterface|Viewport|AddtoViewport _returnvalue_3 0))

(event Collision|EventActorBeginOverlap
  (params (OtherActor :type Actor%20Object%20Reference)))

(event EventTick
  (params (DeltaSeconds :type Float%20%28single-precision%29))
  (if (Variables|Default|GetIsCasting)
    (CallFunction|UpdateCastBar)))

(event EventSpellCastStart
  ;[1 1 1] Spell Cast start
  (UserInterface|Viewport|AddtoViewport (Variables|Default|GetCastBar) 0))

(event EventSpellCastEnd
  ;[1 1 1] Spell cast end
  (Widget|RemovefromParent (Variables|Default|GetCastBar)))

(fn ConstructionScript)